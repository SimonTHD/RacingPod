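; BP_AnakinPod is a player pod for a race, with switchable third- and first-person cameras and a pause menu toggle.
; Input on Z drives the Niagara and two reactor effects, while the gamepad right trigger drives only Niagara.
; A capsule hit sets a collision flag that Tick polls to destroy the pod after a short delay.
; On destruction, PodController respawns it unless the race is complete, having received its start transform at BeginPlay.
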(event OnComponentHit(CapsuleComponent)
  (params (HitComponent :type Primitive%20Component%20Object%20Reference) (OtherActor :type Actor%20Object%20Reference) (OtherComp :type Primitive%20Component%20Object%20Reference) (NormalImpulse :type Vector :default "0, 0, 0") (Hit :type Hit%20Result%20Structure%20%28by%20ref%29))
  (Variables|Default|SetIsCollision? true))

(event Custom|UpdateLap)

(event EventBeginPlay
  (Components|Activation|Deactivate (Variables|Default|GetNiagara))
  (bind _aspod_controller (Utilities|Casting|CastToPodController (Game|GetPlayerController 0)))
  (bind _output_get (Variables|Default|SetControllerReference _aspod_controller))
  (Variables|/Game/Items/PodController.PodController_C|SetRespawnLocation _output_get (Transformation|GetActorTransform)))

(event EventTick
  (params (DeltaSeconds :type Float%20%28single-precision%29))
  ;[1 1 1] Check if player hit the wall
  (bind _playerisstuck_ (CallFunction|RespawnCheck))
  (if _playerisstuck_
    (Utilities|FlowControl|Delay 0.2)
    (Actor|DestroyActor)))

(event EventDestroyed
  (bind _controllerreference (Variables|Default|GetControllerReference))
  ;[1 1 1] Check if player hit the wall
  (if (not (Variables|/Game/Items/PodController.PodController_C|GetRaceComplete _controllerreference))
    (Default|RespawnVehicle _controllerreference)))

(event Input|ActionEvents|InputActionSwitchCamera
  (params (Key :type Key%20Structure :default "None"))
  (:Pressed
    (CallFunction|ChangeCamera)))

(event Input|KeyboardEvents|Z
  (params (Key :type Key%20Structure :default "None"))
  (bind _niagara (Variables|Default|GetNiagara))
  (bind _reacteur (Variables|Default|GetReacteur))
  (bind _reacteur1 (Variables|Default|GetReacteur1))
  (:Pressed
    (Components|Activation|Activate _niagara false)
    (Components|Activation|Activate _reacteur false)
    (Components|Activation|Activate _reacteur1 false))
  (:Released
    (Components|Activation|Deactivate _niagara)
    (Components|Activation|Deactivate _reacteur)
    (Components|Activation|Deactivate _reacteur1)))

(event Input|GamepadEvents|GamepadRightTrigger
  (params (Key :type Key%20Structure :default "None"))
  (bind _niagara (Variables|Default|GetNiagara))
  (:Pressed
    (Components|Activation|Activate _niagara false))
  (:Released
    (Components|Activation|Deactivate _niagara)))

(fn ConstructionScript)

(fn ChangeCamera
  (Components|Activation|ToggleActive (Variables|Default|GetCameraTPS)))

(fn RespawnCheck
  ;[1 1 1] Check if the player need to respawn
  (if (Variables|Default|GetIsCollision?)
    (Variables|Default|SetStuck? true)
    (else
      (Variables|Default|SetStuck? false)))
  (return (Variables|Default|GetStuck?)))

(event Input|ActionEvents|InputActionPauseWidget
  (params (Key :type Key%20Structure))
  (:Pressed
    (Utilities|FlowControl|FlipFlop
      (:A
        (bind _returnvalue (UserInterface|CreateWidget "/Game/Menu2D/pause/PauseMenu.PauseMenu_C"))
        (UserInterface|Viewport|AddtoViewport _returnvalue 0)
        (Game|SetGamePaused true)
        (Variables|/Script/Engine.PlayerController|SetbShowMouseCursor (Game|GetPlayerController 0) true))
      (:B
        (Widget|RemovefromParent _returnvalue)
        (Game|SetGamePaused false)
        (Variables|/Script/Engine.PlayerController|SetbShowMouseCursor (Game|GetPlayerController 0) false)))))